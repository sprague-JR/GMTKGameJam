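; Floor button interactable that tracks whether an actor is standing on it and runs its Interactable Component.
; Overlapping its collider sets a held-down flag and triggers the component immediately, unless a linked push button is assigned.
; With a required push button, it binds to that button's Pushed event and runs the component only if something is overlapping it at that moment.
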(event `self.ReceiveBeginPlay`
  (bind _requiredpushbutton (`self.RequiredPushButton`))
  ;[0.4766 0 1] Event:BeginPlay - Check if pushbutton is required
  (`/Engine/EditorBlueprintResources/StandardMacros.IsValid` _requiredpushbutton
    (:`Is Valid`
      (set `self.bRequiresPushButton` true)
      (add `/Game/_Game/Blueprints/Interactables/Button_Push.Pushed` _requiredpushbutton (delegate `OnPushed`)))))

(event `OnPushed`
  (bind _interactablecomponent (`self.InteractableComponent`))
  ;[0.1953 0 1] Execute Interactable Component
  (if (> (`KismetArrayLibrary.Array_Length` (`self.GetOverlappingActors` null)) 0) :!label _label
    (`/Engine/EditorBlueprintResources/StandardMacros.IsValid` _interactablecomponent
      (:`Is Valid`
        (`/Game/_Game/Blueprints/Interactables/Parent_InteractableComponent.Run` _interactablecomponent)))))

(event `self.Collider.OnComponentBeginOverlap`
  (params (OverlappedComponent :type "PrimitiveComponent Object Reference") (OtherActor :type "Actor Object Reference") (OtherComp :type "PrimitiveComponent Object Reference") (OtherBodyIndex :type Integer) (bFromSweep :type Boolean) (SweepResult :type "HitResult Structure (by ref)"))
  ;[0 1 0.5781] Colliders
  (set `self.bIsHeldDown` true)
  (`/Engine/EditorBlueprintResources/StandardMacros.IsValid` (`self.RequiredPushButton`)
    (:`Is Not Valid`
      (goto _label))))

(event `self.Collider.OnComponentEndOverlap`
  (params (OverlappedComponent :type "PrimitiveComponent Object Reference") (OtherActor :type "Actor Object Reference") (OtherComp :type "PrimitiveComponent Object Reference") (OtherBodyIndex :type Integer))
  ;[0 1 0.5781] Colliders
  (set `self.bIsHeldDown` false))

(fn `UserConstructionScript`)