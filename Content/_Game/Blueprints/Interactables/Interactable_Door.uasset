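; Interactable door that toggles between open and closed each time its Run event fires.
; Run checks IsOpen and calls Open or Close, each of which plays a squeak sound at the actor's location and updates the flag.
; A single timeline drives the yaw of the whole actor, playing forward to open and reversing to close.
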(event `self.Run`
  (if (`self.bIsOpen`)
    (`self.Close`)
    (else
      (`self.Open`))))

(event `Open`
  (`GameplayStatics.PlaySoundAtLocation` "/Game/SeansDebugFolder/Door/DoorSqueak1.DoorSqueak1" (`self.K2_GetActorLocation`) (struct) 1.0 1.0 0.0 null null null)
  (set `self.bIsOpen` true)
  (bind (_direction _doorangle) (`Timeline|OpenTimeline` :!label _label)
    (:`Update`
      (`self.K2_SetActorRotation` (`KismetMathLibrary.MakeRotator` 0.0 0.0 _doorangle)))))

(event `Close`
  (`GameplayStatics.PlaySoundAtLocation` "/Game/SeansDebugFolder/Door/DoorSqueak2.DoorSqueak2" (`self.K2_GetActorLocation`) (struct) 1.0 1.0 0.0 null null null)
  (set `self.bIsOpen` false)
  (goto _label :!via `Reverse`))

(fn `UserConstructionScript`)