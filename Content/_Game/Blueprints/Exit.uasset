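; Exit actor that triggers a game loss once an enemy carrying the eyeball reaches it and its portal finishes opening.
; An overlap with a BP_Enemy that has the eyeball sets an arrival flag.
; Tick then shows the rect light and incrementally stretches the portal plane's Y scale over the door delay.
; When the delay elapses, growth stops and the game-lose call fires, guarded to run only once.
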(event `self.ReceiveTick`
  (params (DeltaSeconds :type "Float (single-precision)"))
  (bind _portalplane (`self.PortalPlane`))
  (bind (_returnvalue_location _returnvalue_rotation _returnvalue_scale) (`KismetMathLibrary.BreakTransform` (`SceneComponent.K2_GetComponentToWorld` _portalplane)))
  (if (`self.bEnemyArrived`)
    (`SceneComponent.SetVisibility` (`self.RectLight`) true false)
    (set `self.TimePassed` (+ DeltaSeconds (`self.TimePassed`)))
    (if (not (`self.bPortalOpened`))
      (`SceneComponent.K2_SetWorldTransform` _portalplane (`KismetMathLibrary.MakeTransform` _returnvalue_location _returnvalue_rotation (+ _returnvalue_scale (`KismetMathLibrary.MakeVector` 0.0 (`KismetMathLibrary.MapRangeClamped` DeltaSeconds 0.0 (`self.DoorDelay`) 0.0 2.0)))) false false)
      (if (>= (`self.TimePassed`) (`self.DoorDelay`))
        (set `self.bPortalOpened` true)
        (if (not (`self.bCalledGameLose`))
          (`self.GameLose`)
          (set `self.bCalledGameLose` true))))))

(event `self.ReceiveActorBeginOverlap`
  (params (OtherActor :type "Actor Object Reference"))
  (bind _asbp_enemy (cast `/Game/_Game/Blueprints/Characters/BP_Enemy` OtherActor))
  (if (`/Game/_Game/Blueprints/Characters/BP_Enemy.has_Eyeball` _asbp_enemy)
    (set `self.bEnemyArrived` true)))

(fn `UserConstructionScript`)