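; Throwable camera pawn that serves as the detached eye of BP_Eyeless, forwarding move, turn, jump and throw input to that character.
; A Tick-driven state machine tracks carried, thrown, moving and stationary phases, gating whether input steers camera or player.
; Pickup and throw events attach or detach it; coming to rest emits AI noise.
; It also supports enemy pickup, velocity-scaled impact sounds and an eased look-at-player turn.
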(event `self.ReceiveBeginPlay`
  (bind _asbp_eyeless (cast `/Game/_Game/Blueprints/Characters/BP_Eyeless` (`self.Player`)))
  (add `/Game/_Game/Blueprints/Characters/BP_Eyeless.PickedUpObject` _asbp_eyeless (delegate `PlayerPickedUp`))
  (add `/Game/_Game/Blueprints/Characters/BP_Eyeless.ThrewObject` _asbp_eyeless (delegate `PlayerThrew`)))

(event `PlayerPickedUp`
  (`self.PlayerPickedUpObject`))

(event `PlayerThrew`
  (`self.PlayerThrewObject`))

(event `self.ReceiveTick`
  (params (DeltaSeconds :type "Float (single-precision)"))
  (switch `CameraState` (`self.CamState`)
    (:`EBeingThrown`
      (`self.CheckMoving`))
    (:`EThrown`
      (`self.CheckStopped`))
    (:`ERotating`
      (`self.LookAtPosition` (`self.K2_GetActorLocation` (`self.Player`)) DeltaSeconds))))

(event `InputAxis|Turn`
  (params (AxisValue :type "Float (single-precision)"))
  (bind _camstate (`self.CamState`))
  ;[0.3125 0 1] Input
  (if (`|EnumEquality` (`self.CamState`) "EStationary")
    (`self.RotateCamera` AxisValue)
    (elif (or (`|EnumEquality` _camstate "ECarried") (`|EnumEquality` _camstate "EBeingThrown"))
      (`self.RotatePlayer` AxisValue))))

(event `InputAxis|MoveRight`
  (params (AxisValue :type "Float (single-precision)"))
  (bind _camstate (`self.CamState`))
  ;[0.3125 0 1] Input
  (if (not (or (`|EnumEquality` _camstate "ECarried") (`|EnumEquality` _camstate "EBeingThrown")))
    (`self.RotatePlayer` AxisValue)))

(event `InputAction|Fire`
  (params (Key :type "Key Structure"))
  ;[0.3125 0 1] Input
  (:`Pressed`
    (bind _asbp_eyeless (cast `/Game/_Game/Blueprints/Characters/BP_Eyeless` (`self.Player`)))
    (`/Engine/EditorBlueprintResources/StandardMacros.IsValid` _asbp_eyeless
      (:`Is Valid`
        (`/Game/_Game/Blueprints/Characters/BP_Eyeless.ThrowPickup` _asbp_eyeless)))))

(event `InputAxis|MoveForward`
  (params (AxisValue :type "Float (single-precision)"))
  ;[0.3125 0 1] Input
  (if (not (`|EnumEquality` (`self.CamState`) "ECarried"))
    (`self.MovePlayer` AxisValue)))

(event `InputAction|Jump`
  (params (Key :type "Key Structure"))
  ;[0.3125 0 1] Input
  (:`Pressed`
    (bind _asbp_eyeless (cast `/Game/_Game/Blueprints/Characters/BP_Eyeless` (`self.Player`)))
    (`Character.Jump` _asbp_eyeless)))

(event `InputAxis|LookUp`
  (params (AxisValue :type "Float (single-precision)"))
  (bind _camstate (`self.CamState`))
  ;[0.3125 0 1] Input
  (if (or (`|EnumEquality` _camstate "ECarried") (`|EnumEquality` _camstate "EStationary"))
    (`self.VerticalLook` AxisValue)))

(event `self.ReceiveHit`
  (params (MyComp :type "PrimitiveComponent Object Reference") (Other :type "Actor Object Reference") (OtherComp :type "PrimitiveComponent Object Reference") (bSelfMoved :type Boolean) (HitLocation :type "Vector Structure") (HitNormal :type "Vector Structure") (NormalImpulse :type "Vector Structure") (Hit :type "HitResult Structure (by ref)"))
  (`GameplayStatics.PlaySoundAtLocation` "/Game/SeansDebugFolder/CameraImpacts/CameraImpact.CameraImpact" HitLocation (struct) (`KismetMathLibrary.Square` (`KismetMathLibrary.FMax` (/ (`KismetMathLibrary.VSize` (`self.GetVelocity`)) 20.0) 1.0)) 1.0 0.0 null null null))

(fn `CheckMoving`
  (if (> (`KismetMathLibrary.VSize` (`SceneComponent.GetComponentVelocity` (`self.SphereCollider`))) 0.0)
    (set `self.CamState` "EThrown")))

(fn `CheckStopped`
  (bind _spherecollider (`self.SphereCollider`))
  (if (< (`KismetMathLibrary.VSize` (`SceneComponent.GetComponentVelocity` _spherecollider)) 0.5)
    (`self.PawnMakeNoise` 0.5 (`SceneComponent.K2_GetComponentLocation` _spherecollider) false null)
    (set `self.CamState` "EStationary")))

(fn `EnemyPickedUp`
  (params (EnemyReference :type "/Game/_Game/Blueprints/Characters/BP_Enemy Object Reference"))
  (if (`|EnumEquality` (`self.CamState`) "EStationary")
    (`self.K2_AttachToActor` EnemyReference "None" "SnapToTarget" "SnapToTarget" "SnapToTarget")
    (`SceneComponent.K2_SetRelativeRotation` :`self` (`self.Camera`))
    (`SceneComponent.K2_SetRelativeLocation` (`self.SphereCollider`) (40.0 0.0 80.0) false true)))

(fn `HasCameraReachedRotationTarget`
  (params (Rotation :type "Rotator Structure"))
  (returns (TargetReached :type Boolean))
  (locals (RotatorDiff :type "Vector Structure"))
  (bind (_returnvalue_roll _returnvalue_pitch _returnvalue_yaw) (`KismetMathLibrary.BreakRotator` (`KismetMathLibrary.NormalizedDeltaRotator` Rotation (`SceneComponent.K2_GetComponentRotation` (`self.Camera`)))))
  (bind _output_get (set `local.RotatorDiff` (`KismetMathLibrary.MakeVector` _returnvalue_roll _returnvalue_pitch _returnvalue_yaw)))
  (return (< (`KismetMathLibrary.VSize` _output_get) (`self.RotationReachedThreshold`))))

(fn `LookAtPosition`
  (params (Position :type "Vector Structure") (DeltaT :type "Float (double-precision)"))
  (locals (TargetRotation :type "Rotator Structure"))
  (bind (_returnvalue_roll _returnvalue_pitch) (`KismetMathLibrary.BreakRotator` (`self.K2_GetActorRotation`)))
  (bind _camera (`self.Camera`))
  (bind (_returnvalue_roll_2 _returnvalue_pitch_2 _returnvalue_yaw) (`KismetMathLibrary.BreakRotator` (`KismetMathLibrary.FindLookAtRotation` (`SceneComponent.K2_GetComponentLocation` (`self.Camera`)) Position)))
  (set `local.TargetRotation` (`KismetMathLibrary.MakeRotator` _returnvalue_roll _returnvalue_pitch _returnvalue_yaw))
  (bind _output_get (set `self.RotationLerpT` (+ DeltaT (`self.RotationLerpT`))))
  (`SceneComponent.K2_SetWorldRotation` _camera (`KismetMathLibrary.RLerp` (`SceneComponent.K2_GetComponentRotation` _camera) (`local.TargetRotation`) (`KismetMathLibrary.Square` _output_get)) false false)
  (bind _targetreached (`self.HasCameraReachedRotationTarget` (`local.TargetRotation`)))
  (if _targetreached
    (set `self.CamState` "EStationary" :!label _label)
    (else
      ;[1 1 1] if this returns false something broke and needs to be fixed
      (if (not (== (`SceneComponent.GetUpVector` (`self.SphereCollider`)) (0.0 0.0 1.0) :`ErrorTolerance` 0.01))
        (`SceneComponent.K2_SetWorldRotation` (`self.Camera`) (`local.TargetRotation`) false false)
        (goto _label)))))

(fn `MovePlayer`
  (params (MovementDirection :type "Float (double-precision)"))
  (bind _player (`self.Player`))
  (`/Engine/EditorBlueprintResources/StandardMacros.IsValid` _player
    (:`Is Valid`
      (bind _asbp_eyeless (cast `/Game/_Game/Blueprints/Characters/BP_Eyeless` _player))
      (set `/Game/_Game/Blueprints/Characters/BP_Eyeless.Speed` MovementDirection _asbp_eyeless)
      (`MovementComponent.K2_MoveUpdatedComponent` (`self.GetComponentByClass` _player "/Script/Engine.CharacterMovementComponent") (* (`KismetMathLibrary.Normal` (`self.GetActorForwardVector` _player)) (* MovementDirection (`self.PlayerMovementSpeed`))) (`self.K2_GetActorRotation` _player) true false))))

(fn `PlayerPickedUpObject`
  (if (not (`|EnumEquality` (`self.CamState`) "ECarried"))
    (bind _asbp_eyeless (cast `/Game/_Game/Blueprints/Characters/BP_Eyeless` (`self.Player`)))
    (if (== (`/Game/_Game/Blueprints/Characters/BP_Eyeless.Pickup` _asbp_eyeless) self)
      (`GameplayStatics.PlaySoundAtLocation` "/Game/SeansDebugFolder/PickupEye/PickupEye.PickupEye" (`self.K2_GetActorLocation`) (struct) 1.0 1.0 0.0 null null null)
      (set `self.CamState` "ECarried")
      (`PrimitiveComponent.SetSimulatePhysics` (`self.SphereCollider`) false)
      (bind _asbp_eyeless_2 (cast `/Game/_Game/Blueprints/Characters/BP_Eyeless` (`self.Player`)))
      (`self.K2_AttachToActor` _asbp_eyeless_2 "None" "SnapToTarget" "SnapToTarget" "KeepRelative")
      (`SceneComponent.K2_SetRelativeRotation` :`self` (`self.Camera`))
      (`self.K2_SetActorRelativeLocation` (45.0 0.0 60.0) false true))))

(fn `PlayerThrewObject`
  (bind _camera (`self.Camera`))
  (bind _asbp_eyeless (cast `/Game/_Game/Blueprints/Characters/BP_Eyeless` (`self.Player`)))
  (if (== (`/Game/_Game/Blueprints/Characters/BP_Eyeless.Pickup` _asbp_eyeless) self)
    (`self.K2_DetachFromActor` "KeepWorld" "KeepRelative" "KeepWorld")
    (`SceneComponent.K2_SetWorldRotation` _camera (`self.K2_GetActorRotation` (`self.Player`)) false false)
    (`SceneComponent.K2_AddLocalRotation` _camera (struct :`Yaw` 90.0) false false)
    (set `self.CamState` "EBeingThrown")))

(fn `RotateCamera`
  (params (A :type "Float (double-precision)"))
  (`SceneComponent.K2_AddLocalRotation` (`self.Camera`) (`KismetMathLibrary.MakeRotator` 0.0 0.0 (* A (`self.RotationSpeed`))) false false))

(fn `RotatePlayer`
  (params (Rotation :type "Float (double-precision)"))
  (bind _player (`self.Player`))
  (`/Engine/EditorBlueprintResources/StandardMacros.IsValid` _player
    (:`Is Valid`
      (`self.K2_AddActorWorldRotation` _player (`KismetMathLibrary.MakeRotator` 0.0 0.0 (* Rotation (`self.PlayerRotationSpeed`))) false false))))

(fn `ThrowCamera`
  (bind _spherecollider (`self.SphereCollider`))
  (`PrimitiveComponent.AddForce` _spherecollider (+ (* (`KismetMathLibrary.Normal` (`KismetMathLibrary.GetForwardVector` (`SceneComponent.K2_GetComponentRotation` _spherecollider))) -1000.0) (0.0 0.0 5000.0)) "None" false))

(fn `UserConstructionScript`)

(fn `VerticalLook`
  (params (Rate :type "Float (double-precision)"))
  (bind (_relativerotation_roll _relativerotation_pitch _relativerotation_yaw) (`KismetMathLibrary.BreakRotator` (`SceneComponent.RelativeRotation` (`self.Camera`))))
  (`SceneComponent.K2_SetRelativeRotation` (`self.Camera`) (`KismetMathLibrary.MakeRotator` 0.0 (`KismetMathLibrary.FClamp` (+ _relativerotation_pitch (* Rate -1.0)) -70.0 70.0) _relativerotation_yaw) false false))