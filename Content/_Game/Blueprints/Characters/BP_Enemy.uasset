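; BP_Enemy is a patrolling enemy that seeks noises and carries the player's detachable eyeball camera to the level Exit.
; PawnSensing hearing resets a Boredom timer, so Tick moves it to the last noise until bored, then to its PatrolPoint.
; Overlapping a loose eye away from the player stuns it if the eye is moving under physics.
; Otherwise, an unbored enemy grabs it and, after a delay, heads for the Exit.
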(event `OnPickUpEye`
  ;[0 0.1328 1] Event:BeginPlay - Set up references to player and exits
  (set `self.has_Eyeball` true))

(event `self.ReceiveBeginPlay`
  (bind _patrol_point (`self.patrol_point`))
  ;[0 0.1328 1] Event:BeginPlay - Set up references to player and exits
  (`|ExecutionSequence`
    (:`then_0`
      (bind _outactors (`GameplayStatics.GetAllActorsOfClass` "/Game/_Game/Blueprints/Characters/CameraBlueprint.CameraBlueprint_C"))
      (bind _output_get (set `self.CameraReference` (`|GetArrayItem` _outactors)))
      (add `/Game/_Game/Blueprints/Characters/CameraBlueprint.PickupEye` _output_get (delegate `OnPickUpEye`)))
    (:`then_1`
      (bind _outactors_2 (`GameplayStatics.GetAllActorsOfClass` "/Game/_Game/Blueprints/Exit.Exit_C"))
      (set `self.ExitLocation` (`self.K2_GetActorLocation` (`|GetArrayItem` _outactors_2)))
      (set `self.StartPos` (`self.K2_GetActorLocation`))
      (`/Engine/EditorBlueprintResources/StandardMacros.IsValid` _patrol_point
        (:`Is Valid`
          (set `self.Goal` (`self.K2_GetActorLocation` _patrol_point)))))))

(event `self.ReceiveTick`
  (params (DeltaSeconds :type "Float (single-precision)"))
  (bind _returnvalue (`self.GetController` self))
  ;[0 1 0.7188] Event:Tick - Patrolling Logic
  (if (not (`self.isStunned`))
    (if (`self.has_Eyeball`)
      (`|ExecutionSequence`
        (:`then_0`
          (`/Game/_Game/Blueprints/Characters/CameraBlueprint.EnemyPickedUp` (`self.CameraReference`) self))
        (:`then_1`
          (bind _output_get (set `self.TimePassed` (+ DeltaSeconds (`self.TimePassed`))))
          (if (>= _output_get 1.0)
            (set `self.JustPickedUp` false)
            (`AIBlueprintHelperLibrary.SimpleMoveToLocation` _returnvalue (`self.ExitLocation`)))))
      (else
        (bind _output_get_2 (set `self.boredom` (`KismetMathLibrary.FMin` (+ DeltaSeconds (`self.boredom`)) 50000.0)))
        (if (< _output_get_2 (`self.boredom_threshold`))
          (`AIBlueprintHelperLibrary.SimpleMoveToLocation` _returnvalue (`self.last_noise_location`))
          (else
            (`AIBlueprintHelperLibrary.SimpleMoveToLocation` _returnvalue (`self.K2_GetActorLocation` (`self.patrol_point`)))))))
    (else
      (bind _output_get_3 (set `self.StunTime` (+ (`self.StunTime`) DeltaSeconds)))
      (if (> _output_get_3 (`self.StunThreshold`))
        (set `self.StunTime` 0.0)
        (set `self.isStunned` false)
        (else
          (`MovementComponent.StopMovementImmediately` (`self.CharacterMovement`)))))))

(event `self.ReceiveActorBeginOverlap`
  (params (OtherActor :type "Actor Object Reference"))
  (if (not (`self.isStunned`))
    (bind _ascamera_blueprint (cast `/Game/_Game/Blueprints/Characters/CameraBlueprint` OtherActor))
    (if (not (`|EnumEquality` (`CameraPawn.CamState` _ascamera_blueprint) "ECarried"))
      (bind _spherecollider (`/Game/_Game/Blueprints/Characters/CameraBlueprint.SphereCollider` _ascamera_blueprint))
      (if (< (`KismetMathLibrary.Vector_Distance` (`self.K2_GetActorLocation` (`/Game/_Game/Blueprints/Characters/CameraBlueprint.Player` _ascamera_blueprint)) (`SceneComponent.K2_GetComponentLocation` _spherecollider)) 200.0)
        _
        (elif (`SceneComponent.IsSimulatingPhysics` _spherecollider "None")
          (if (> (`KismetMathLibrary.VSize` (`SceneComponent.GetComponentVelocity` _spherecollider)) 1.0)
            (set `self.isStunned` true)
            (else
              (if (< (`self.boredom`) (`self.boredom_threshold`)) :!label _label
                (set `self.has_Eyeball` true)
                (set `self.JustPickedUp` true))))
          (else
            (goto _label)))))))

(event `self.PawnSensing.OnHearNoise`
  (params (Instigator :type "Pawn Object Reference") (Location :type "Vector Structure (by ref)") (Volume :type "Float (single-precision)"))
  (if (not (`self.isStunned`))
    (`self.hear_noise` Location)))

(fn `hear_noise`
  (params (noise_location :type "Vector Structure"))
  (set `self.boredom` 0.0)
  (set `self.last_noise_location` noise_location))

(fn `UserConstructionScript`)