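; BP_Eyeless is a character with health, landing noise, and the ability to pick up and throw objects.
; It makes pawn noise when a fall ends and calls the Die dispatcher when damage depletes health.
; Capsule overlap immediately picks up the other actor; ThrowPickup enables physics on its PhysicsCollider-tagged component and applies forward and upward force.
; Pickup and throw fire dispatchers, while the hold-position update logic is disconnected and never runs.
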(event `self.ReceiveBeginPlay`
  (set `self.Health` (`self.MaxHealth`)))

(event `self.ReceiveTick`
  (params (DeltaSeconds :type "Float (single-precision)"))
  (if (and (`self.was_falling`) (not (`NavMovementComponent.IsFalling` (`self.CharacterMovement`))))
    (`self.PawnMakeNoise` 1.0 (0.0 0.0 0.0) true null))
  (set `self.was_falling` (`NavMovementComponent.IsFalling` (`self.CharacterMovement`))))

(event `self.ReceiveAnyDamage`
  (params (Damage :type "Float (single-precision)") (DamageType :type "DamageType Object Reference") (InstigatedBy :type "Controller Object Reference") (DamageCauser :type "Actor Object Reference"))
  (bind _output_get (set `self.Health` (- (`self.Health`) Damage)))
  (if (<= _output_get 0.0)
    (`self.Die`)
    (elif (>= _output_get (`self.MaxHealth`))
      (set `self.Health` (`self.MaxHealth`)))))

(event `self.CapsuleComponent.OnComponentBeginOverlap`
  (params (OverlappedComponent :type "PrimitiveComponent Object Reference") (OtherActor :type "Actor Object Reference") (OtherComp :type "PrimitiveComponent Object Reference") (OtherBodyIndex :type Integer) (bFromSweep :type Boolean) (SweepResult :type "HitResult Structure (by ref)"))
  (`/Engine/EditorBlueprintResources/StandardMacros.IsValid` (`self.GetComponentByClass` "/Script/Engine.ShapeComponent")
    (:`Is Valid`
      (set `self.Pickup` OtherActor)
      (`self.PickupObject`))))

(event `self.CapsuleComponent.OnComponentEndOverlap`
  (params (OverlappedComponent :type "PrimitiveComponent Object Reference") (OtherActor :type "Actor Object Reference") (OtherComp :type "PrimitiveComponent Object Reference") (OtherBodyIndex :type Integer))
  (bind _pickup (`self.Pickup`))
  (`/Engine/EditorBlueprintResources/StandardMacros.IsValid` _pickup
    (:`Is Valid`
      (if (== OtherActor _pickup)
        (set `self.Pickup` null)))))

(fn `GetPickupHoldLocation`
  (returns (Location :type "Vector Structure"))
  (return (+ (`self.K2_GetActorLocation`) (* (`KismetMathLibrary.Normal` (`self.GetActorForwardVector`)) (`self.HoldDistance`)))))

(fn `PickupObject`
  (`/Engine/EditorBlueprintResources/StandardMacros.IsValid` (`self.Pickup`)
    (:`Is Valid`
      (set `self.HoldingPickup` true)
      (`self.PickedUpObject`))))

(fn `ThrowPickup`
  (bind _pickup (`self.Pickup`))
  (if (`self.HoldingPickup`)
    (`/Engine/EditorBlueprintResources/StandardMacros.IsValid` _pickup
      (:`Is Valid`
        (`self.ThrewObject`)
        (set `self.HoldingPickup` false)
        (`/Engine/EditorBlueprintResources/StandardMacros.IsValid` _pickup
          (:`Is Valid`
            (bind _asshape_component (cast `ShapeComponent` (`|GetArrayItem` (`self.GetComponentsByTag` _pickup "/Script/Engine.ActorComponent" "PhysicsCollider"))))
            (`/Engine/EditorBlueprintResources/StandardMacros.IsValid` _asshape_component
              (:`Is Valid`
                (`PrimitiveComponent.SetSimulatePhysics` _asshape_component true)
                (`PrimitiveComponent.AddForce` _asshape_component (+ (* (`KismetMathLibrary.Normal` (`self.GetActorForwardVector` self)) (`self.ThrowForce`)) (`KismetMathLibrary.MakeVector` 0.0 0.0 (`self.ThrowForceUp`))) "None" false)))))))))

(fn `UserConstructionScript`)